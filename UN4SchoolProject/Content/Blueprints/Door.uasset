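; Door actor that swings by driving its relative yaw from the DoorRotation timeline.
; Actors tagged AI entering TriggerBox play the timeline automatically; any other overlapping actor enables player 0's input on the door.
; With input enabled, F toggles DoorStatus and plays or reverses the timeline.
; Any actor leaving the box disables that input, with no check on who left.
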(event `self.TriggerBox.OnComponentBeginOverlap`
  (params (OverlappedComponent :type "PrimitiveComponent Object Reference") (OtherActor :type "Actor Object Reference") (OtherComp :type "PrimitiveComponent Object Reference") (OtherBodyIndex :type Integer) (bFromSweep :type Boolean) (SweepResult :type "HitResult Structure (by ref)"))
  (if (`self.ActorHasTag` OtherActor "AI")
    (set `self.DoorStatus` false :!label _label)
    (bind (_direction _doorrot) (`Timeline|DoorRotation` :!label _label_2)
      (:`Update`
        (`self.K2_SetActorRelativeRotation` (`KismetMathLibrary.MakeRotator` 0.0 0.0 _doorrot))))
    (else
      (`self.EnableInput` (`GameplayStatics.GetPlayerController` 0)))))

(event `Key|F`
  (params (Key :type "Key Structure"))
  (:`Pressed`
    (if (`self.DoorStatus`)
      (goto _label)
      (else
        (set `self.DoorStatus` true)
        (goto _label_2 :!via `Reverse`)))))

(event `self.TriggerBox.OnComponentEndOverlap`
  (params (OverlappedComponent :type "PrimitiveComponent Object Reference") (OtherActor :type "Actor Object Reference") (OtherComp :type "PrimitiveComponent Object Reference") (OtherBodyIndex :type Integer))
  (`self.DisableInput` (`GameplayStatics.GetPlayerController` 0)))

(fn `UserConstructionScript`)