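; AITestGameMode is a game mode Blueprint that keeps an elapsed-time counter in Minutes and Seconds variables.
; Tick feeds a one-second Delay, which acts as a throttle so Seconds increments roughly once per second.
; Minutes increments and Seconds resets to zero only once Seconds exceeds 60, so each counted minute spans 61 increments.
; BeginPlay and the construction script are empty.
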(event `self.ReceiveTick`
  (params (DeltaSeconds :type "Float (single-precision)"))
  ;[1 1 1] Timer
  (`KismetSystemLibrary.Delay` 1.0)
  (set `self.Seconds` (+ (`self.Seconds`) 1))
  (if (> (`self.Seconds`) 60)
    (set `self.Minutes` (+ (`self.Minutes`) 1))
    (set `self.Seconds` 0)))

(fn `UserConstructionScript`)